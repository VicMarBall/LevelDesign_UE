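; BP_ProjectileTarget_GetPoint is a test target actor that reacts when a projectile hits it.
; OnProjectileHit prints a "Get Point Hit" message and spawns the FXS_DoorDestroyed effect at the impact point, oriented along the surface normal.
; Despite the name, it contains no scoring logic, and its BeginPlay, overlap and Tick events are disabled placeholders.
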(event `self.OnProjectileHit`
  (params (Hit :type "HitResult Structure"))
  (`KismetSystemLibrary.PrintString` "Get Point Hit")
  (`NiagaraFunctionLibrary.SpawnSystemAtLocation` "/Game/BlueprintsTesting/VFXs/FXS_DoorDestroyed.FXS_DoorDestroyed" Hit_Location (`KismetMathLibrary.Conv_VectorToRotator` Hit_Normal)))

(fn `UserConstructionScript`
  (`parent.UserConstructionScript`))