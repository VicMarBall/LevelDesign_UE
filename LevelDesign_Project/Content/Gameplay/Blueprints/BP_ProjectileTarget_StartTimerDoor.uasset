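; A projectile target that starts the player's timer when shot, named as the start timer door.
; On a projectile hit it prints a debug string and spawns the door-destroyed effect at the impact point, oriented along the surface normal.
; It then casts player 0's character to BP_FirstPersonCharacter and sets IsTimerActivated, leaving the timer itself to that character.
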(event `self.OnProjectileHit`
  (params (Hit :type "HitResult Structure"))
  (`KismetSystemLibrary.PrintString` "Start Timer Hit")
  (`NiagaraFunctionLibrary.SpawnSystemAtLocation` "/Game/Gameplay/VFXs/FXS_DoorDestroyed.FXS_DoorDestroyed" Hit_Location (`KismetMathLibrary.Conv_VectorToRotator` Hit_Normal))
  (bind _asbp_first_person_character (cast `/Game/FirstPerson/Blueprints/BP_FirstPersonCharacter` (`GameplayStatics.GetPlayerCharacter` 0)))
  (set `/Game/FirstPerson/Blueprints/BP_FirstPersonCharacter.IsTimerActivated` true _asbp_first_person_character))

(fn `UserConstructionScript`
  (`parent.UserConstructionScript`))